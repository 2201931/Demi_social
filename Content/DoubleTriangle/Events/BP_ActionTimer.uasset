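; Action timer Blueprint meant to fire a separate event for each minute from 0 to 10.
; StartTimer sets a looping one-second timer by function name, and TimerTick increments CurrentTime on each tick.
; The switch on elapsed minutes is unconnected, so TimerTick triggers no minute events.
; The first three minute events only print debug strings, the rest are empty, and nothing shown calls StartTimer.
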(event Custom|StartTimer
  ;[0 0 0] StartTimer connects to Event BeginPlay to start the timer and to Set Timer by Function Name to start ticking every second.
  ; TimerTick connects to Set CurrentTime to update the time, and Set CurrentTime connects to the Switch on Int to determine which minute event should be triggered.
  (Utilities|Time|SetTimerbyFunctionName 0 "TimerTick" 1.0 true)
  (Development|PrintString "start"))

(event Custom|TimerTick
  ;[0 0 0] StartTimer connects to Event BeginPlay to start the timer and to Set Timer by Function Name to start ticking every second.
  ; TimerTick connects to Set CurrentTime to update the time, and Set CurrentTime connects to the Switch on Int to determine which minute event should be triggered.
  (bind _output_get (Variables|Default|SetCurrentTime (+ (Variables|Default|GetCurrentTime) 1.0))))

(event Custom|OnMinute_0
  ;[0 0 0] StartTimer connects to Event BeginPlay to start the timer and to Set Timer by Function Name to start ticking every second.
  ; TimerTick connects to Set CurrentTime to update the time, and Set CurrentTime connects to the Switch on Int to determine which minute event should be triggered.
  (Development|PrintString "Hello"))

(event Custom|OnMinute_2
  ;[0 0 0] StartTimer connects to Event BeginPlay to start the timer and to Set Timer by Function Name to start ticking every second.
  ; TimerTick connects to Set CurrentTime to update the time, and Set CurrentTime connects to the Switch on Int to determine which minute event should be triggered.
  (Development|PrintString "2"))

(event Custom|OnMinute_4)

(event Custom|OnMinute_3)

(event Custom|OnMinute_5)

(event Custom|OnMinute_8)

(event Custom|OnMinute_1
  ;[0 0 0] StartTimer connects to Event BeginPlay to start the timer and to Set Timer by Function Name to start ticking every second.
  ; TimerTick connects to Set CurrentTime to update the time, and Set CurrentTime connects to the Switch on Int to determine which minute event should be triggered.
  (Development|PrintString "1"))

(event Custom|OnMinute_6)

(event Custom|OnMinute_7)

(event Custom|OnMinute_10)

(event Custom|OnMinute_9)