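; BP_Timer is a game clock that triggers numbered "minute" events for scheduling character actions.
; From BeginPlay, a looping named-function timer increments CurrentTime every three seconds, and a switch on its floored value selects a minute event from zero to ten.
; The minute one and two handlers invoke CallTimer on BP_Bartender and BP_Flynn actors respectively.
; Minute zero only prints, later handlers are empty, and their draft nodes are unconnected.
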(event Custom|StartTimer
  ;[0 0 0] StartTimer connects to Event BeginPlay to start the timer and to Set Timer by Function Name to start ticking every second.
  ; TimerTick connects to Set CurrentTime to update the time, and Set CurrentTime connects to the Switch on Int to determine which minute event should be triggered.
  (Utilities|Time|SetTimerbyFunctionName 0 "TimerTick" 3.0 true)
  (Development|PrintString "start"))

(event Custom|TimerTick
  ;[0 0 0] StartTimer connects to Event BeginPlay to start the timer and to Set Timer by Function Name to start ticking every second.
  ; TimerTick connects to Set CurrentTime to update the time, and Set CurrentTime connects to the Switch on Int to determine which minute event should be triggered.
  (bind _output_get (Variables|Default|SetCurrentTime (+ (Variables|Default|GetCurrentTime) 1.0)))
  (switch int (Math|Float|Floor _output_get)
    (:0
      (CallFunction|OnMinute0))
    (:1
      (CallFunction|OnMinute1))
    (:2
      (CallFunction|OnMinute2))
    (:3
      (CallFunction|OnMinute3))
    (:4
      (CallFunction|OnMinute4))
    (:5
      (CallFunction|OnMinute5))
    (:6
      (CallFunction|OnMinute6))
    (:7
      (CallFunction|OnMinute7))
    (:8
      (CallFunction|OnMinute8))
    (:9
      (CallFunction|OnMinute9))
    (:10
      (CallFunction|OnMinute10))))

(event Custom|OnMinute_0
  ;[0 0 0] StartTimer connects to Event BeginPlay to start the timer and to Set Timer by Function Name to start ticking every second.
  ; TimerTick connects to Set CurrentTime to update the time, and Set CurrentTime connects to the Switch on Int to determine which minute event should be triggered.
  (Development|PrintString "Hello"))

(event Custom|OnMinute_2
  ;[0 0 0] StartTimer connects to Event BeginPlay to start the timer and to Set Timer by Function Name to start ticking every second.
  ; TimerTick connects to Set CurrentTime to update the time, and Set CurrentTime connects to the Switch on Int to determine which minute event should be triggered.
  (bind _outactors (Actor|GetAllActorsOfClass "/Game/Saira/Blueprints/BP_Flynn.BP_Flynn_C"))
  (Default|CallTimer _outactors)
  (Development|PrintString "2"))

(event Custom|OnMinute_4)

(event Custom|OnMinute_3)

(event Custom|OnMinute_5)

(event Custom|OnMinute_8)

(event Custom|OnMinute_1
  ;[0 0 0] StartTimer connects to Event BeginPlay to start the timer and to Set Timer by Function Name to start ticking every second.
  ; TimerTick connects to Set CurrentTime to update the time, and Set CurrentTime connects to the Switch on Int to determine which minute event should be triggered.
  (bind _outactors (Actor|GetAllActorsOfClass "/Game/Saira/Blueprints/BP_Bartender.BP_Bartender_C"))
  (Default|CallTimer _outactors)
  (Development|PrintString "1"))

(event Custom|OnMinute_6)

(event Custom|OnMinute_7)

(event Custom|OnMinute_10)

(event Custom|OnMinute_9)

(event EventBeginPlay
  (CallFunction|StartTimer))

(fn ConstructionScript)