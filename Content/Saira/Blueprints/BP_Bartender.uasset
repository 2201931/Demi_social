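; Bartender NPC that walks to the player to take an order through a Convai chatbot, then returns to the bar.
; BeginPlay binds the order event to a timer; on reaching the player, a narrative trigger makes the bartender ask for the order with voice and actions.
; A fixed timer then fires a goodbye trigger and, after a short delay, moves the bartender to a hardcoded bar location.
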(event Custom|GetOrder
  (Development|PrintString "Bartender Getting Order")
  (AI|AIMoveTo self (Transformation|GetActorLocation (Game|GetPlayerCharacter 0)) 0 1e+02 false
    (:OnSuccess
      (Class|ConvaiChatbotComponent|ExecuteNarrativeTrigger (Variables|Default|GetConvaiChatbot) "Take my order" 0 true true false)
      (Utilities|Time|SetTimerbyFunctionName 0 "GoBack" 15.0))))

(event Custom|GoBack
  (Development|PrintString "Bartender go back to bar")
  (Class|ConvaiChatbotComponent|ExecuteNarrativeTrigger (Variables|Default|GetConvaiChatbot) "Goodbye!" 0 true true false)
  (Utilities|FlowControl|Delay 6.0)
  (AI|AIMoveTo self "1757.009619,-2797.500000,0.000000" 0 5.0 false))

(event EventBeginPlay
  (EventDispatchers|BindEventtoTimer (delegate Custom|GetOrder)))

(fn ConstructionScript)